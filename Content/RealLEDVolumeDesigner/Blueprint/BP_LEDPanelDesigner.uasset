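; Editor tool actor that designs LED panels and bakes their pixel-map textures for RealLEDVolumeDesigner.
; Step 1 loads a manual config or the preset DataTable's first row, derives pixel pitch, and rebuilds a scaled grid of instanced LED pixels.
; Step 2 saves the capture render target as an HDR static texture with post process temporarily enabled, named after the panel, with a timestamp on name clashes.
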(event `(Step 1) - Update Panel (Build)`
  (bind _led_panel_configuration___preset (`self.LED Panel Configuration - Preset`))
  (bind _led_panel_configuration_selected (`self.LED Panel Configuration Selected`))
  (bind _led_panel_configuration___manual (`self.LED Panel Configuration - Manual`))
  (bind ((`LEDPixel_Diameter_24_1789D0B04DC6AAAC29E59E9129EF6EB7` _ledpixel_diameter) (`LEDPanel_Resolution_H_7_29DE5F9E4F975DE8BE9EB985BC2FC1DF` _ledpanel_resolution_h) (`LEDPanel_Resolution_V_9_1B4E8D3940A07967BA6F9C83486BF051` _ledpanel_resolution_v) (`LEDPanel_Width_2_5F244BBE4EBA0CCF10EF1980A8BE08F3` _ledpanel_width) (`LEDPanel_Height_4_05C784CF4A2C1A567A647F8CF5118AF2` _ledpanel_height)) (break `/Game/RealLEDVolumeDesigner/Blueprint/Struct/S_LEDPanel_Config` _led_panel_configuration_selected))
  (bind ((`LEDPanel_MaxBrightness_38_E2AAB4EF45ABA809F905BCB8EA1A5885` _ledpanel_maxbrightness) (`LEDPanel_Resolution_H_7_29DE5F9E4F975DE8BE9EB985BC2FC1DF` _ledpanel_resolution_h_2) (`LEDPanel_Width_2_5F244BBE4EBA0CCF10EF1980A8BE08F3` _ledpanel_width_2)) (break `/Game/RealLEDVolumeDesigner/Blueprint/Struct/S_LEDPanel_Config` _led_panel_configuration___manual))
  (bind _returnvalue (/ _ledpanel_width _ledpanel_height))
  (bind _returnvalue_2 (`KismetMathLibrary.Conv_DoubleToVector` _ledpixel_diameter))
  (bind _returnvalue_3 (/ 500.0 _ledpanel_width))
  (bind _returnvalue_4 (/ _ledpixel_diameter 10.0))
  (bind _returnvalue_5 (/ _ledpanel_width (`KismetMathLibrary.Conv_IntToDouble` _ledpanel_resolution_h)))
  (bind _returnvalue_6 (/ (- (/ _returnvalue_5 10.0) _returnvalue_4) 2.0))
  (bind _returnvalue_7 (`EditorDialogLibrary.ShowMessage` "Info" "Ready to generate LED panel based on your specifications. \n \nThis may take a few moments or longer depending on your \nhardware specifications, please be patient. \n \nOnce completed don't forget to save your texture \nusing the Step 2 button and add it to your custom preset asset. \n \nDo you want to continue?" "OkCancel" "Ok" "Info"))
  (switch `EAppReturnType` _returnvalue_7
    (:`Cancel`
      (`EditorDialogLibrary.ShowMessage` "Info" "LED Panel generation cancelled." "Ok" "Ok" "Info"))
    (:`Ok`
      (`InstancedStaticMeshComponent.ClearInstances` (`self.LEDPixels`))
      (`self.K2_SetActorLocation` self (0.0 0.0 0.0) false false)
      ;[1 1 1] Load Settings
      (switch `/Game/RealLEDVolumeDesigner/Blueprint/Enum/E_LEDPanel_PresetNames` (`self.LED Panel Configuration`)
        (:`NewEnumerator0`
          (bind _structout (setmembers `/Game/RealLEDVolumeDesigner/Blueprint/Struct/S_LEDPanel_Config` :`StructRef` _led_panel_configuration___manual :`LEDPixel_Calculated_Pitch` (/ _ledpanel_width_2 (`KismetMathLibrary.Conv_IntToDouble` _ledpanel_resolution_h_2))))
          (set `self.LED Panel Configuration - Manual` _structout)
          (set `self.LED Panel Configuration Selected` _led_panel_configuration___manual)
          ;[1 1 1] Generate
          (bind _structout_2 (setmembers `/Game/RealLEDVolumeDesigner/Blueprint/Struct/S_LEDPanel_Config` :`StructRef` _led_panel_configuration_selected :`LEDPixel_Calculated_Pitch` _returnvalue_5 :!label _label))
          (set `self.LED Panel Configuration Selected` _structout_2)
          (`SceneComponent.K2_SetRelativeLocation` (`self.LEDPixels`) (`KismetMathLibrary.MakeVector` _returnvalue_6 (* (+ _returnvalue_6 _returnvalue_4) _returnvalue)) false false)
          (for _index (range _ledpanel_resolution_h)
            (bind _returnvalue_8 (* (`KismetMathLibrary.Conv_IntToDouble` _index) (/ _returnvalue_5 10.0)))
            (`InstancedStaticMeshComponent.AddInstance` (`self.LEDPixels`) (`KismetMathLibrary.MakeTransform` (`KismetMathLibrary.MakeVector` _returnvalue_8) (struct) _returnvalue_2) false)
            (for _index_2 (range _ledpanel_resolution_v)
              (`InstancedStaticMeshComponent.AddInstance` (`self.LEDPixels`) (`KismetMathLibrary.MakeTransform` (`KismetMathLibrary.MakeVector` _returnvalue_8 (* (`KismetMathLibrary.Conv_IntToDouble` _index_2) (/ _returnvalue_5 10.0))) (struct) _returnvalue_2) false)))
          (`SceneComponent.SetRelativeScale3D` (`self.LEDPixels`) (`KismetMathLibrary.MakeVector` _returnvalue_3 (* _returnvalue _returnvalue_3) 1.0)))
        (:`NewEnumerator1`
          (`/Engine/EditorBlueprintResources/StandardMacros.IsValid` _led_panel_configuration___preset
            (:`Is Valid`
              (bind _outrownames (`DataTableFunctionLibrary.GetDataTableRowNames` _led_panel_configuration___preset))
              (bind _returnvalue_9 (`|GetDataTableRow` _led_panel_configuration___preset (`|GetArrayItem` _outrownames))
                (:`then`
                  (set `self.LED Panel Configuration Selected` _returnvalue_9)
                  (bind ((`LEDPanel_MaxBrightness_38_E2AAB4EF45ABA809F905BCB8EA1A5885` _ledpanel_maxbrightness_2) (`LEDPanel_Resolution_H_7_29DE5F9E4F975DE8BE9EB985BC2FC1DF` _ledpanel_resolution_h_3) (`LEDPanel_Width_2_5F244BBE4EBA0CCF10EF1980A8BE08F3` _ledpanel_width_3)) (break `/Game/RealLEDVolumeDesigner/Blueprint/Struct/S_LEDPanel_Config` _returnvalue_9))
                  (bind _structout_3 (setmembers `/Game/RealLEDVolumeDesigner/Blueprint/Struct/S_LEDPanel_Config` :`StructRef` _returnvalue_9 :`LEDPixel_Calculated_Pitch` (/ _ledpanel_width_3 (`KismetMathLibrary.Conv_IntToDouble` _ledpanel_resolution_h_3))))
                  (set `self.LED Panel Configuration Selected` _structout_3)
                  (goto _label))
                (:`RowNotFound`
                  (`KismetSystemLibrary.PrintString` null "Error: No data found in preset" true true (struct :`R` 1.0 :`A` 1.0)))))
            (:`Is Not Valid`
              (`KismetSystemLibrary.PrintString` null "First select a Preset asset"))))))))

(event `(Step 2) - Save Generated Pixel Map Texture`
  (bind _panelname (break `/Game/RealLEDVolumeDesigner/Blueprint/Struct/S_LEDPanel_Config` (`self.LED Panel Configuration Selected`)))
  (bind (_year _month _day _hour _minute _second) (`KismetMathLibrary.BreakDateTime` (`KismetMathLibrary.Now`)))
  (bind _returnvalue (`KismetStringLibrary.Concat_StrStr` "LEDPanel_PixelMap_" (`KismetTextLibrary.Conv_TextToString` _panelname)))
  ;[1 1 1] Generate Map
  (set `PostProcessComponent.bEnabled` true (`self.PostProcess`))
  (bind _returnvalue_2 (`KismetRenderingLibrary.RenderTargetCreateStaticTexture2DEditorOnly` "/Game/RealLEDVolumeDesigner/Blueprint/RT_LEDPanel_Capture.RT_LEDPanel_Capture" (`KismetSystemLibrary.GetDisplayName` (`self.CaptureCamera`)) "TC_HDR"))
  (set `Texture.LODGroup` "TEXTUREGROUP_EffectsNotFiltered" _returnvalue_2)
  (bind _output_get (set `self.GeneratedLEDPanelTexture` _returnvalue_2))
  (bind _returnvalue_3 (`EditorAssetLibrary.GetPathNameForLoadedAsset` _output_get))
  (bind _returnvalue_4 (`EditorAssetLibrary.DoesAssetExist` (`KismetTextLibrary.Conv_TextToString` (`|FormatText` "{path}/{name}.{name}" (`KismetStringLibrary.Split` _returnvalue_3 "/" "IgnoreCase" "FromEnd") (`KismetStringLibrary.Concat_StrStr` "LEDPanel_PixelMap_" (`KismetTextLibrary.Conv_TextToString` _panelname))))))
  (if _returnvalue_4
    (`EditorUtilityLibrary.RenameAsset` _output_get (`KismetStringLibrary.Concat_StrStr` _returnvalue "_" (`KismetTextLibrary.Conv_TextToString` (`|FormatText` "{year}{month}{day}-{hour}{minute}{second}" (`KismetStringLibrary.GetSubstring` (`KismetStringLibrary.Conv_IntToString` _year) 2 2) _month _day _hour _minute _second))))
    (`KismetSystemLibrary.PrintString` null "An asset with this name already exists in this location, appending date and time" true true (struct :`R` 1.0 :`G` 0.318576 :`A` 1.0) 10.0)
    (else
      (`EditorUtilityLibrary.RenameAsset` _output_get _returnvalue)
      (`KismetSystemLibrary.PrintString` null (`KismetTextLibrary.Conv_TextToString` (`|FormatText` "Pixel Map created successfully with name \"{name}\"" _returnvalue)) true true (struct :`G` 1.0 :`A` 1.0) 5.0)))
  (set `PostProcessComponent.bEnabled` false (`self.PostProcess`)))

(fn `UserConstructionScript`)
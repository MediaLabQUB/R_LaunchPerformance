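; Editor-time generator actor that builds nDisplay static mesh assets for an LED volume in Build mode, then destroys itself.
; After confirmation, Geometry Script creates a panel grid from supplied vertices with two UV sets.
; Column ranges become per-node polygroups, named panels are deleted, and the mesh is split by group.
; Each section gets renormalised UV0, is saved as an asset and optionally replaces previously spawned, tagged scene actors.
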(event `self.OnRebuildGeneratedMesh`
  (params (TargetMesh :type "DynamicMesh Object Reference"))
  (bind _ledpanelcolumnrangestonodes (`self.LEDPanelColumnRangesToNodes`))
  (bind _ndisplaymeshsectionvertices (`self.NDisplayMeshSectionVertices`))
  (bind _spawnedbyobject (`self.SpawnedByObject`))
  (bind _ndisplaymeshsectionprefix (`self.NDisplayMeshSectionPrefix`))
  (bind _panelstoremove (`self.PanelsToRemove`))
  (bind _polygrouptonode (`self.PolygroupToNode`))
  (switch `/Game/RealLEDVolumeDesigner/Blueprint/Enum/E_LEDVolume_Mode` (`self.LEDVolume_Mode`)
    (:`NewEnumerator0`
      (`EditorDialogLibrary.ShowMessage` "LED Volume Designer - Warning" "LED Volume Mode must be set to \"Build\" \nin order to generate nDisplay meshes." "Ok" "No")
      (`self.Exit`))
    (:`NewEnumerator1`
      (if (< (`KismetArrayLibrary.Array_Length` (`self.LEDPanelColumnRangesToNodes`)) 1)
        (`EditorDialogLibrary.ShowMessage` "LED Volume Designer - Warning" "First create some LED column-range-to-node entries in the \nGenerate nDisplay Mesh Settings section to define which columns of LED Panels are assigned to which nDisplay nodes. \n \nThere is an example set on the LED wall array in the Demonstraiton map." "Ok" "No")
        (`self.Exit`)
        (else
          (bind _returnvalue (`EditorDialogLibrary.ShowMessage` "LED Volume Designer - Information" (`|FormatText` "Continuing will generate {sectionCount} Static Mesh assets \nin {path} with the name of {prefix}_[INDEX] \n \nExisting assets in this location will be overwritten! \n \nWould you like to continue?" (`KismetArrayLibrary.Array_Length` (`self.LEDPanelColumnRangesToNodes`)) (`self.NDisplayMeshSectionsExportPath`) (`self.NDisplayMeshSectionPrefix`)) "OkCancel" "Cancel"))
          (switch `EAppReturnType` _returnvalue
            (:`No`
              (`self.Exit` :!label _label))
            (:`Yes`
              (if (`self.bHasCompleted`) :!label _label_2
                (set `self.bFrozen` true)
                (else
                  (set `self.Target Mesh` TargetMesh)
                  (bind _returnvalue_2 (`DynamicMesh.Reset` TargetMesh))
                  (bind _returnvalue_3 (`GeometryScriptLibrary_MeshPolygroupFunctions.EnablePolygroups` _returnvalue_2 null))
                  (bind _returnvalue_4 (`GeometryScriptLibrary_MeshPolygroupFunctions.ClearPolygroups` _returnvalue_3 (struct) 0 null))
                  (bind _returnvalue_5 (`GeometryScriptLibrary_MeshPrimitiveFunctions.AppendRectangleXY` _returnvalue_4 (make `GeometryScriptPrimitiveOptions` "PerQuad") (`KismetMathLibrary.MakeTransform` (0.0 0.0 0.0)) (`self.LEDArrayWidth`) (`self.LEDArrayHeight`) (+ (`self.LEDPanelColumns`) 1) (+ (`self.LEDPanelRows`) 1) null))
                  (bind _returnvalue_6 (`GeometryScriptLibrary_MeshUVFunctions.SetNumUVSets` _returnvalue_5 2 null))
                  (bind _returnvalue_7 (`GeometryScriptLibrary_MeshUVFunctions.CopyUVSet` _returnvalue_6 0 1 null))
                  (if (> (`KismetArrayLibrary.Array_Length` _ndisplaymeshsectionvertices) 0)
                    (for (_array_element _array_index) _ndisplaymeshsectionvertices
                      (`GeometryScriptLibrary_MeshBasicEditFunctions.SetVertexPosition` _returnvalue_7 _array_index _array_element)))
                  ;[1 1 1] UV Channel 1
                  (bind _returnvalue_8 (`GeometryScriptLibrary_MeshUVFunctions.ScaleMeshUVs` _returnvalue_7 1 (1.0 1.0) (0.0 0.0) (struct) null))
                  (bind _returnvalue_9 (`GeometryScriptLibrary_MeshUVFunctions.TranslateMeshUVs` _returnvalue_8 1 (`KismetMathLibrary.MakeVector2D` 0.0 (- 0.5 (/ (`.Y` (`KismetMathLibrary.BreakVector2D` (`.Max` (break `Box2D` (`.ReturnValue` (`GeometryScriptLibrary_MeshQueryFunctions.GetUVSetBoundingBox` _returnvalue_8 1)))))) 2.0))) (struct) null))
                  (bind _returnvalue_10 (`GeometryScriptLibrary_MeshUVFunctions.ScaleMeshUVs` _returnvalue_9 1 (-1.0 1.0) (0.5 0.5) (struct) null))
                  ;[1 1 1] Generate node groups
                  (for (_array_element_2 _array_index_2) (`self.LEDPanelColumnRangesToNodes`)
                    (`KismetArrayLibrary.Array_Clear` _polygrouptonode)
                    (for _index (range (`self.LEDPanelRows`))
                      (bind (_autonamethisnode _ndisplaynodename _startcolumn _endcolumn) (break `/Game/RealLEDVolumeDesigner/Blueprint/Struct/S_LEDVolume_ColumnRangeToNode` _array_element_2))
                      (bind _returnvalue_11 (- _startcolumn 1))
                      (for _index_2 (range (+ (- (- _endcolumn 1) _returnvalue_11) 1))
                        (`KismetArrayLibrary.Array_Add` _polygrouptonode (+ (+ (+ _index_2 (* _index (`self.LEDPanelColumns`))) _returnvalue_11) 1))))
                    (bind (_selection _returnvalue_12) (`GeometryScriptLibrary_MeshSelectionFunctions.ConvertIndexArrayToMeshSelection` _returnvalue_10 (`self.PolygroupToNode`) "Polygroups"))
                    (bind _output_get (set `self.Selection` _selection))
                    (`GeometryScriptLibrary_MeshPolygroupFunctions.SetPolygroupForMeshSelection` _returnvalue_12 (struct) _output_get (+ _array_index_2 1))
                    (if _autonamethisnode
                      (bind _structout (setmembers `/Game/RealLEDVolumeDesigner/Blueprint/Struct/S_LEDVolume_ColumnRangeToNode` :`StructRef` (`|GetArrayItem` _ledpanelcolumnrangestonodes _array_index_2) :`NDisplay Node Name` (`KismetStringLibrary.Concat_StrStr` "NDisplayNode_" (`KismetStringLibrary.Conv_IntToString` _array_index_2))))
                      (`KismetArrayLibrary.Array_Set` _ledpanelcolumnrangestonodes _array_index_2 _structout)))
                  (if (> (`KismetArrayLibrary.Array_Length` _panelstoremove) 0)
                    (for _array_element_3 _panelstoremove
                      (bind _returnvalue_13 (`KismetStringLibrary.GetSubstring` _array_element_3 0 (`KismetMathLibrary.SelectInt` 2 1 (> (`self.LEDPanelRows`) 26))))
                      (if (not (`KismetStringLibrary.IsEmpty` _returnvalue_13))
                        (bind (_value _returnvalue_14) (`BlueprintMapLibrary.Map_Find` (`self.LetterToNumberMap`) _returnvalue_13))
                        (if _returnvalue_14
                          (bind (_lefts _rights) (`KismetStringLibrary.Split` _array_element_3 _returnvalue_13))
                          (if (`KismetStringLibrary.IsNumeric` _rights)
                            (bind _returnvalue_15 (+ (* _value (* (`self.LEDPanelColumns`) 2)) (* (- (`KismetStringLibrary.Conv_StringToInt` _rights) 1) 2)))
                            (`GeometryScriptLibrary_MeshBasicEditFunctions.DeleteTriangleFromMesh` (`self.Target Mesh`) _returnvalue_15)
                            (`GeometryScriptLibrary_MeshBasicEditFunctions.DeleteTriangleFromMesh` (`self.Target Mesh`) (+ _returnvalue_15 1)))))))
                  (bind _componentmeshes (`GeometryScriptLibrary_MeshDecompositionFunctions.SplitMeshByPolygroups` (`self.Target Mesh`) (struct) (`self.Mesh Pool`) null))
                  (`KismetArrayLibrary.Array_Clear` (`self.NDisplayMeshSections`))
                  (for (_array_element_4 _array_index_3) _componentmeshes
                    (bind (_bisvaliduvset _buvsetisempty _returnvalue_16) (`GeometryScriptLibrary_MeshQueryFunctions.GetUVSetBoundingBox` _array_element_4))
                    ;[1 1 1] UVChannel 0
                    (bind _returnvalue_17 (`GeometryScriptLibrary_MeshUVFunctions.TranslateMeshUVs` _array_element_4 0 (`KismetMathLibrary.MakeVector2D` (* (`KismetMathLibrary.BreakVector2D` (break `Box2D` _returnvalue_16)) -1.0) (* (`.Y` (`KismetMathLibrary.BreakVector2D` (break `Box2D` _returnvalue_16))) -1.0)) (struct) null))
                    (if (or (> (- 1.0 (`KismetMathLibrary.BreakVector2D` (`.Max` (break `Box2D` _returnvalue_16)))) 0.0) (> (- 1.0 (`.Y` (`KismetMathLibrary.BreakVector2D` (`.Max` (break `Box2D` _returnvalue_16))))) 0.0))
                      (bind _returnvalue_18 (`GeometryScriptLibrary_MeshUVFunctions.ScaleMeshUVs` _returnvalue_17 0 (`KismetMathLibrary.MakeVector2D` (/ 1.0 (`KismetMathLibrary.BreakVector2D` (`.Max` (break `Box2D` (`.ReturnValue` (`GeometryScriptLibrary_MeshQueryFunctions.GetUVSetBoundingBox` _returnvalue_17)))))) 1.0) (0.0 0.0) (struct) null))
                      (`GeometryScriptLibrary_MeshUVFunctions.ScaleMeshUVs` _returnvalue_18 0 (`KismetMathLibrary.MakeVector2D` 1.0 (/ 1.0 (`.Y` (`KismetMathLibrary.BreakVector2D` (`.Max` (break `Box2D` (`.ReturnValue` (`GeometryScriptLibrary_MeshQueryFunctions.GetUVSetBoundingBox` (`self.Target Mesh`))))))))) (0.0 0.0) (struct) null))
                    (bind _returnvalue_19 (`GeometryScriptLibrary_CreateNewAssetFunctions.CreateNewStaticMeshAssetFromMesh` _array_element_4 (`KismetTextLibrary.Conv_TextToString` (`|FormatText` "{path}{name}_{index}" (`self.NDisplayMeshSectionsExportPath`) _ndisplaymeshsectionprefix _array_index_3)) (make `GeometryScriptCreateNewStaticMeshAssetOptions` false) null)
                      (:`Failure`
                        (`KismetSystemLibrary.PrintString` "Generating Mesh Sections Failed - Check export path valid and contains trailing forward slash" true true (struct :`R` 1.0 :`B` 0.00845 :`A` 1.0)))
                      (:`Success`
                        (`KismetSystemLibrary.PrintString` (`KismetTextLibrary.Conv_TextToString` (`|FormatText` "Generating Mesh Section {name}_{index} Success" _ndisplaymeshsectionprefix _array_index_3)) true true (struct :`R` 0.047693 :`G` 0.171875 :`B` 0.031331 :`A` 1.0) 5.0)
                        (`/Engine/EditorBlueprintResources/StandardMacros.IsValid` _returnvalue_19
                          (:`Is Valid`
                            (`KismetArrayLibrary.Array_Add` (`self.NDisplayMeshSections`) _returnvalue_19))))))
                  ;[1 1 1] Add To Scene
                  (if (and (> (`KismetArrayLibrary.Array_Length` (`self.NDisplayMeshSections`)) 0) (`self.bAddMeshSectionsToScene`))
                    (bind _outactors (`GameplayStatics.GetAllActorsWithTag` (`KismetStringLibrary.Conv_StringToName` (`KismetStringLibrary.Concat_StrStr` (`self.SpawnedByObject`) "_" "NDisplayMeshSection"))))
                    (for _array_element_5 _outactors
                      (`self.K2_DestroyActor` _array_element_5))
                    (for (_array_element_6 _array_index_4) (`self.NDisplayMeshSections`)
                      (bind _returnvalue_20 (`|SpawnActorFromClass` "/Script/Engine.StaticMeshActor" (`self.LEDVolumeTransform`) "AlwaysSpawn" "OverrideRootScale" null null))
                      (bind _staticmeshcomponent (`StaticMeshActor.StaticMeshComponent` _returnvalue_20))
                      (`StaticMeshComponent.SetStaticMesh` _staticmeshcomponent _array_element_6)
                      (`PrimitiveComponent.SetMaterial` _staticmeshcomponent 0 "/Game/RealLEDVolumeDesigner/Materials/M_LEDVolume_NDisplayMeshSections.M_LEDVolume_NDisplayMeshSections")
                      (set `Actor.Tags` (`|MakeArray` (`KismetStringLibrary.Conv_StringToName` (`KismetStringLibrary.Concat_StrStr` _spawnedbyobject "_" "NDisplayMeshSection"))) _returnvalue_20)
                      (`self.SetActorLabel` _returnvalue_20 (`KismetStringLibrary.Concat_StrStr` _spawnedbyobject "_" (`self.NDisplayMeshSectionPrefix`) "_" (`KismetStringLibrary.Conv_IntToString` _array_index_4)) false))
                    (else
                      (`EditorDialogLibrary.ShowMessage` "LED Volume Designer - Information" "Generation Complete! \n \nIt is highly recommended to set 'Use Full Precision UVs' on the mesh sections in the Static Mesh viewer details panel." "Ok" "No")))
                  (set `self.bHasCompleted` true :!label _label_3)
                  (set `self.bFrozen` true)
                  (`DynamicMeshPool.FreeAllMeshes` (`self.Mesh Pool`))
                  (`self.ReleaseAllComputeMeshes`)
                  (`self.K2_DestroyActor`))))
            (:`YesAll`
              (goto _label_2))
            (:`NoAll`
              (goto _label))
            (:`Cancel`
              (goto _label))
            (:`Ok`
              (goto _label_2))
            (:`Retry`
              (goto _label))
            (:`Continue`
              (goto _label_2))))))))

(event `Exit`
  ;[1 1 1] Add To Scene
  (goto _label_3))

(fn `UserConstructionScript`)